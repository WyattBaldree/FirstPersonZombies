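; EscapeFloat is an actor Blueprint that makes its Diety component bob up and down.
; BeginPlay stores the component's world location as the resting point.
; Each Tick adds delta time to a counter and sets the component's world Z to that point plus the counter's sine scaled by FloatAmount, with X and Y fixed.
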(event `self.ReceiveBeginPlay`
  (set `self.DefaultLocation` (`SceneComponent.K2_GetComponentLocation` (`self.Diety`))))

(event `self.ReceiveTick`
  (params (DeltaSeconds :type "Float (single-precision)"))
  (set `self.Counter` (+ DeltaSeconds (`self.Counter`)))
  (`SceneComponent.K2_SetWorldLocation` (`self.Diety`) (`KismetMathLibrary.MakeVector` (.x (`self.DefaultLocation`)) (.y (`self.DefaultLocation`)) (+ (.z (`self.DefaultLocation`)) (* (`KismetMathLibrary.Sin` (`self.Counter`)) (`self.FloatAmount`)))) false false))

(fn `UserConstructionScript`)