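; Exit actor that shows key progress with three point lights and tells the player character when it is at the exit.
; It binds to the character's KeyActive event at BeginPlay; each call reveals the next hidden light, starts that light's InterpToMovement and increments Count.
; Begin and end overlap set and clear AtExit on the FPS character.
; Count is not read here beyond its increment.
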(event `self.ReceiveBeginPlay`
  (add `/Game/Assets/Blueprints/FPSCharacter_bp.KeyActive` (cast `/Game/Assets/Blueprints/FPSCharacter_bp` (`GameplayStatics.GetPlayerCharacter` 0) :!pure true) (delegate `KeyActive_Event_0`)))

(event `KeyActive_Event_0`
  (bind _interptomovement (`self.InterpToMovement`))
  (bind _pointlight1 (`self.PointLight1`))
  (bind _interptomovement1 (`self.InterpToMovement1`))
  (bind _pointlight2 (`self.PointLight2`))
  (bind _interptomovement2 (`self.InterpToMovement2`))
  (bind _pointlight (`self.PointLight`))
  (if (not (`SceneComponent.IsVisible` _pointlight))
    (`SceneComponent.ToggleVisibility` _pointlight true)
    (`MovementComponent.SetUpdatedComponent` _interptomovement _pointlight)
    (`ActorComponent.Activate` _interptomovement false)
    (bind _result (`/Engine/EditorBlueprintResources/StandardMacros.IncrementInt` (`self.Count`) :!label _label)
      (:`  `
        (set `self.Count` _result)))
    (elif (not (`SceneComponent.IsVisible` _pointlight1))
      (`SceneComponent.ToggleVisibility` _pointlight1 true)
      (`MovementComponent.SetUpdatedComponent` _interptomovement1 _pointlight1)
      (`ActorComponent.Activate` _interptomovement1 false)
      (goto _label)
      (elif (not (`SceneComponent.IsVisible` _pointlight2))
        (`SceneComponent.ToggleVisibility` _pointlight2 true)
        (`MovementComponent.SetUpdatedComponent` _interptomovement2 _pointlight2)
        (`ActorComponent.Activate` _interptomovement2 false)
        (goto _label)))))

(event `self.ReceiveActorBeginOverlap`
  (params (OtherActor :type "Actor Object Reference"))
  (bind _asfpscharacter_bp (cast `/Game/Assets/Blueprints/FPSCharacter_bp` OtherActor))
  (set `/Game/Assets/Blueprints/FPSCharacter_bp.AtExit` true _asfpscharacter_bp))

(event `self.ReceiveActorEndOverlap`
  (params (OtherActor :type "Actor Object Reference"))
  (bind _asfpscharacter_bp (cast `/Game/Assets/Blueprints/FPSCharacter_bp` OtherActor))
  (set `/Game/Assets/Blueprints/FPSCharacter_bp.AtExit` false _asfpscharacter_bp))

(fn `UserConstructionScript`)