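; Repairable window actor that gains wooden boards while the player holds the interact key.
; InteractBegin and InteractEnd reset the timers and flags; Tick waits out InteractDelay, then adds one board per BoardDelay, the first almost immediately.
; Board count lives in the skeletal mesh's AnimBlueprint as NumBoards, zeroed on BeginPlay and incremented without an upper limit here.
; Tick also prints both timers every frame for debugging.
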(event `self.ReceiveBeginPlay`
  (`self.SetInteractString` "Hold E to repair")
  (bind _aswood_plank_window_skeleton_anim_blueprint (cast `/Game/Assets/Mesh/WindowPlanks/WoodPlankWindow_Skeleton_AnimBlueprint` (`SkeletalMeshComponent.GetAnimInstance` (`self.SkeletalMesh`))))
  (bind _output_get (set `self.MyWindow` _aswood_plank_window_skeleton_anim_blueprint))
  (set `/Game/Assets/Mesh/WindowPlanks/WoodPlankWindow_Skeleton_AnimBlueprint.NumBoards` 0 _output_get))

(event `self.ReceiveTick`
  (params (DeltaSeconds :type "Float (single-precision)"))
  (bind _mywindow (`self.MyWindow`))
  (`KismetSystemLibrary.PrintString` (`KismetStringLibrary.Concat_StrStr` "InteractDelayCurrent: " (`KismetStringLibrary.Conv_DoubleToString` (`self.InteractDelayCurrent`)) " / " (`KismetStringLibrary.Conv_DoubleToString` (`self.InteractDelay`))))
  (`KismetSystemLibrary.PrintString` (`KismetStringLibrary.Concat_StrStr` "BoardDelayCurrent: " (`KismetStringLibrary.Conv_DoubleToString` (`self.BoardDelayCurrent`)) " / " (`KismetStringLibrary.Conv_DoubleToString` (`self.BoardDelay`))))
  (if (`self.Interacting`)
    (if (`self.Repairing`)
      (bind _output_get (set `self.BoardDelayCurrent` (+ DeltaSeconds (`self.BoardDelayCurrent`))))
      (if (> _output_get (`self.BoardDelay`))
        (set `self.BoardDelayCurrent` (- (`self.BoardDelayCurrent`) (`self.BoardDelay`)))
        (bind _result (`/Engine/EditorBlueprintResources/StandardMacros.IncrementInt` (`/Game/Assets/Mesh/WindowPlanks/WoodPlankWindow_Skeleton_AnimBlueprint.NumBoards` _mywindow))
          (:`  `
            (set `/Game/Assets/Mesh/WindowPlanks/WoodPlankWindow_Skeleton_AnimBlueprint.NumBoards` _result _mywindow))))
      (else
        (bind _output_get_2 (set `self.InteractDelayCurrent` (+ DeltaSeconds (`self.InteractDelayCurrent`))))
        (if (> _output_get_2 (`self.InteractDelay`))
          (set `self.Repairing` true))))))

(event `self.InteractBegin`
  (set `self.InteractDelayCurrent` 0.0)
  (set `self.Repairing` false)
  (set `self.BoardDelayCurrent` (`self.BoardDelay`))
  (set `self.Interacting` true))

(event `self.InteractEnd`
  (set `self.InteractDelayCurrent` 0.0)
  (set `self.Repairing` false)
  (set `self.BoardDelayCurrent` 0.0)
  (set `self.Interacting` false))

(fn `UserConstructionScript`)