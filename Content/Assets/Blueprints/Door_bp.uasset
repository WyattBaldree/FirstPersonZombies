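; Purchasable double door that the player pays to operate through interaction.
; On BeginPlay it builds the price prompt, caches the skeletal mesh's DoubleDoors anim Blueprint and sets its initial Open state.
; InteractBegin calls DoTransaction on the interacting FPSCharacter_bp with Price and, on success, toggles the anim Blueprint's Open flag, so closing also costs the price.
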(event `self.ReceiveBeginPlay`
  (`self.SetInteractString` (`KismetStringLibrary.Concat_StrStr` "$" (`KismetStringLibrary.Conv_IntToString` (`self.Price`)) " To Open."))
  (bind _asdouble_doors_skeleton_anim_blueprint (cast `/Game/Assets/Mesh/DoubleDoor/DoubleDoors_Skeleton_AnimBlueprint` (`SkeletalMeshComponent.GetAnimInstance` (`self.SkeletalMesh`))))
  (bind _output_get (set `self.MyDoor` _asdouble_doors_skeleton_anim_blueprint))
  (set `/Game/Assets/Mesh/DoubleDoor/DoubleDoors_Skeleton_AnimBlueprint.Open` (`self.Open`) _output_get))

(event `self.InteractBegin`
  (params (InteractingActor :type "Actor Object Reference"))
  (bind _mydoor (`self.MyDoor`))
  (bind _asfpscharacter_bp (cast `/Game/Assets/Blueprints/FPSCharacter_bp` InteractingActor))
  (bind _returnvalue (`FPSCharacter.DoTransaction` _asfpscharacter_bp (`self.Price`)))
  (if _returnvalue
    (set `/Game/Assets/Mesh/DoubleDoor/DoubleDoors_Skeleton_AnimBlueprint.Open` (not (`/Game/Assets/Mesh/DoubleDoor/DoubleDoors_Skeleton_AnimBlueprint.Open` _mydoor)) _mydoor)))

(fn `UserConstructionScript`)