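; Money pickup Blueprint that adds cash to the player when touched.
; On overlap with an FPSCharacter_bp, it adds its Value to that character's Cash, calls UpdateCash with the new total and destroys itself.
; The construction script sets its static mesh from the Mesh variable, so each instance can have its own look.
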(event `self.ReceiveActorBeginOverlap`
  (params (OtherActor :type "Actor Object Reference"))
  (bind _asfpscharacter_bp (cast `/Game/Assets/Blueprints/FPSCharacter_bp` OtherActor))
  (bind _output_get (set `/Game/Assets/Blueprints/FPSCharacter_bp.Cash` (+ (`/Game/Assets/Blueprints/FPSCharacter_bp.Cash` _asfpscharacter_bp) (`self.Value`)) _asfpscharacter_bp))
  (`/Game/Assets/Blueprints/FPSCharacter_bp.UpdateCash` _asfpscharacter_bp _output_get)
  (`self.K2_DestroyActor`))

(fn `UserConstructionScript`
  (`parent.UserConstructionScript`)
  (`StaticMeshComponent.SetStaticMesh` (`self.StaticMesh`) (`self.Mesh`)))