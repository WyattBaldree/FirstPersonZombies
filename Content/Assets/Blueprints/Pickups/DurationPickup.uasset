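; Duration-based powerup pickup that activates when an FPSCharacter_bp overlaps it.
; It identifies its type by matching its display name against the E_DurationPowerups enum names, then XOR-toggles the corresponding bit in the character's Powerups bitmask.
; The matching PowerupsData row supplies an image and duration for the HUD, after which the pickup destroys itself.
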(event `self.ReceiveActorBeginOverlap`
  (params (OtherActor :type "Actor Object Reference"))
  (bind _asfpscharacter_bp (cast `/Game/Assets/Blueprints/FPSCharacter_bp` OtherActor))
  (bind _enumvalue (foreach `/Game/Assets/Blueprints/E_DurationPowerups`)
    (:`LoopBody`
      (bind _returnvalue (`|GetEnumeratorNameAsString` _enumvalue))
      (if (`KismetStringLibrary.EqualEqual_StrStr` _returnvalue (`KismetSystemLibrary.GetDisplayName` self))
        (set `/Game/Assets/Blueprints/FPSCharacter_bp.Powerups` (`KismetMathLibrary.Xor_IntInt` (`/Game/Assets/Blueprints/FPSCharacter_bp.Powerups` _asfpscharacter_bp) (`KismetMathLibrary.FTrunc` (`KismetMathLibrary.MultiplyMultiply_FloatFloat` 2.0 (`KismetMathLibrary.Conv_ByteToDouble` _enumvalue)))) _asfpscharacter_bp)
        (bind _returnvalue_2 (`|GetDataTableRow` "/Game/Assets/Blueprints/Pickups/PowerupsData.PowerupsData" (`KismetStringLibrary.Conv_StringToName` _returnvalue))
          (:`then`
            (`/Game/Assets/UMG/FPSHUD_bp.AddImage` (`/Game/Assets/Blueprints/FPSCharacter_bp.HUD` _asfpscharacter_bp) (`.Image_12_5107536F4B3CDE20B67BFAB1971B39A9` (break `/Game/Assets/Blueprints/Pickups/PowerupsStruct` _returnvalue_2)) (`KismetMathLibrary.Conv_IntToDouble` (`.Duration_8_C81C1DE94BDF3812C0C14B9271B12FAD` (break `/Game/Assets/Blueprints/Pickups/PowerupsStruct` _returnvalue_2))))
            (`self.K2_DestroyActor`)))))))

(fn `UserConstructionScript`
  (`parent.UserConstructionScript`))