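; Ammo pickup that refills the held weapon's reserve ammo when an FPSCharacter_bp overlaps it.
; It adds two magazines' worth, capped at the reserve maximum, then destroys itself.
; With a full reserve but a partly empty magazine, it adds the missing rounds to the reserve beyond that cap and is still consumed.
; If both are full, the pickup remains in place.
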(event `self.ReceiveActorBeginOverlap`
  (params (OtherActor :type "Actor Object Reference"))
  (bind _asfpscharacter_bp (cast `/Game/Assets/Blueprints/FPSCharacter_bp` OtherActor))
  (bind _heldweapon (`FPSCharacter.HeldWeapon` _asfpscharacter_bp))
  (bind _ammocurrent (`Weapon.AmmoCurrent` _heldweapon))
  (bind _ammomax (`Weapon.AmmoMax` _heldweapon))
  (if (< _ammocurrent _ammomax)
    (bind _magazinemax (`Weapon.MagazineMax` _heldweapon))
    (bind _returnvalue (+ _ammocurrent (* _magazinemax 2)))
    (if (> _returnvalue _ammomax)
      (set `Weapon.AmmoCurrent` _ammomax _heldweapon)
      (else
        (set `Weapon.AmmoCurrent` _returnvalue _heldweapon)))
    (`self.K2_DestroyActor` :!label _label)
    (else
      (bind _magazinecurrent (`Weapon.MagazineCurrent` _heldweapon))
      (if (< _magazinecurrent _magazinemax)
        (set `Weapon.AmmoCurrent` (+ _ammocurrent (- _magazinemax _magazinecurrent)) _heldweapon)
        (goto _label)))))

(fn `UserConstructionScript`
  (`parent.UserConstructionScript`))