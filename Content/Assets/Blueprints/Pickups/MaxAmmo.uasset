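; Max ammo pickup that refills all of the player character's weapons when touched.
; On actor overlap it casts to FPSCharacter_bp, then loops through that character's Weapons array and sets each valid weapon's magazine and ammo counts to their maximums.
; The pickup destroys itself after the refill, and overlaps by other actor types are ignored.
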(event `self.ReceiveActorBeginOverlap`
  (params (OtherActor :type "Actor Object Reference"))
  (bind _asfpscharacter_bp (cast `/Game/Assets/Blueprints/FPSCharacter_bp` OtherActor))
  (for _array_element (`FPSCharacter.Weapons` _asfpscharacter_bp)
    (`/Engine/EditorBlueprintResources/StandardMacros.IsValid` _array_element
      (:`Is Valid`
        (set `Weapon.MagazineCurrent` (`Weapon.MagazineMax` _array_element) _array_element)
        (set `Weapon.AmmoCurrent` (`Weapon.AmmoMax` _array_element) _array_element))))
  (`self.K2_DestroyActor`))

(fn `UserConstructionScript`
  (`parent.UserConstructionScript`))