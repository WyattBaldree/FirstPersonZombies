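; FPSZombie_bp is a zombie enemy that chases its target and melee-attacks the player.
; Tick reissues AIMoveTo toward TargetActor at a fixed interval and counts down an attack cooldown while alive, spawned and not attacking.
; When cooled down and overlapping the player, AttackStart waits out a windup, rechecks state, then damages FPSCharacter_bp.
; Die spawns an item through the GameMode's loot manager before calling the parent Die.
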(event `self.ReceiveBeginPlay`)

(event `self.ReceiveTick`
  (params (DeltaSeconds :type "Float (single-precision)"))
  (bind _attackcurrent (`self.AttackCurrent`))
  (`|ExecutionSequence`
    (:`then_0`
      ;[1 1 1] Once Per Second
      (bind _output_get (set `self.CurrentDelta` (+ DeltaSeconds (`self.CurrentDelta`))))
      (if (>= _output_get (`self.UpdateInterval`))
        (`|ExecutionSequence`
          (:`then_0`
            (set `self.CurrentDelta` (- (`self.CurrentDelta`) (`self.UpdateInterval`))))
          (:`then_1`
            ;[1 1 1] Path To Destination
            (`|AIMoveTo` self (0.0 0.0 0.0) (`self.TargetActor`))))))
    (:`then_1`
      (if (and (`|EnumInequality` (`self.ZombieState`) "VE_Spawning") (`|EnumInequality` (`self.ZombieState`) "VE_Dead") (not (`self.Attacking`)))
        (set `self.AttackCurrent` (- _attackcurrent DeltaSeconds))
        (if (and (<= _attackcurrent 0.0) (`self.IsOverlappingActor` (`GameplayStatics.GetPlayerPawn` 0)))
          (`self.AttackStart`))))))

(event `AttackStart`
  (set `self.Attacking` true)
  (`KismetSystemLibrary.Delay` (`self.AttackDelay`))
  (set `self.AttackCurrent` (`self.AttackInterval`))
  (if (and (`|EnumInequality` (`self.ZombieState`) "VE_Spawning") (`|EnumInequality` (`self.ZombieState`) "VE_Dead"))
    (`/Game/Assets/Blueprints/FPSCharacter_bp.TakeDamage` (cast `/Game/Assets/Blueprints/FPSCharacter_bp` (`GameplayStatics.GetPlayerCharacter` 0) :!pure true) (`self.DealDamage`))
    (`KismetSystemLibrary.Delay` (- (`self.AttackLength`) (`self.AttackDelay`)))
    (set `self.Attacking` false)
    (else
      (set `self.Attacking` false))))

(event `self.ReceiveActorBeginOverlap`
  (params (OtherActor :type "Actor Object Reference")))

(event `self.ReceiveActorEndOverlap`
  (params (OtherActor :type "Actor Object Reference")))

(fn `Die`
  (returns (ReturnValue :type Boolean))
  (`/Game/Assets/Blueprints/LootManager_bp.SpawnItem` (cast `/Game/Assets/Blueprints/LootManager_bp` (`FirstPersonZombiesGameMode.MyLootManager` (cast `/Game/Assets/Blueprints/FirstPersonZombiesGameMode_bp` (`GameplayStatics.GetGameMode`) :!pure true)) :!pure true) (`self.GetTransform`))
  (bind _returnvalue (`parent.Die`))
  (return _returnvalue))

(fn `UserConstructionScript`)