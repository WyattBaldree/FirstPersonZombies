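; WeaponShop_bp is a weapon shop actor that detects when an FPS character enters or leaves its area.
; On begin overlap it sets the character's AtShop flag and marks PlayerOwned if either of the character's first two weapons matches the shop's WeaponClass.
; On end overlap it clears both AtShop and PlayerOwned.
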(event `self.ReceiveActorBeginOverlap`
  (params (OtherActor :type "Actor Object Reference"))
  (bind _weaponclass (`self.WeaponClass`))
  (bind _asfpscharacter_bp (cast `/Game/Assets/Blueprints/FPSCharacter_bp` OtherActor))
  (set `/Game/Assets/Blueprints/FPSCharacter_bp.AtShop` true _asfpscharacter_bp)
  (bind _weapons (`FPSCharacter.Weapons` _asfpscharacter_bp))
  (set `self.PlayerOwned` (or (== (`GameplayStatics.GetObjectClass` (`|GetArrayItem` _weapons)) _weaponclass) (== _weaponclass (`GameplayStatics.GetObjectClass` (`|GetArrayItem` _weapons 1))))))

(event `self.ReceiveActorEndOverlap`
  (params (OtherActor :type "Actor Object Reference"))
  (bind _asfpscharacter_bp (cast `/Game/Assets/Blueprints/FPSCharacter_bp` OtherActor))
  (set `/Game/Assets/Blueprints/FPSCharacter_bp.AtShop` false _asfpscharacter_bp)
  (set `self.PlayerOwned` false))

(fn `UserConstructionScript`)