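; Player character Blueprint for a first-person shooter with purchasable doors and weapons, keystones and an escape exit.
; Tick drives held-weapon fire, health regeneration after a damage cooldown, and timed expiry of bitmask powerups, two of which modify cash transactions.
; Interact buys doors, which spawn random hallways or, every third time, dead-end rooms, and handles shop weapons or ammo, keystones and the exit.
; It also manages weapon switching and HUD, pause, completion and game-over widgets.
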(event `self.ReceiveBeginPlay`
  (bind _returnvalue (`|CreateWidget` "/Game/Assets/UMG/PauseMenu_bp.PauseMenu_bp_C"))
  (set `self.PauseMenu` _returnvalue)
  (bind _returnvalue_2 (`|CreateWidget` "/Game/Assets/UMG/Completed.Completed_C"))
  (set `self.Complete` _returnvalue_2)
  (bind _returnvalue_3 (`|CreateWidget` "/Game/Assets/UMG/GameOver.GameOver_C"))
  (set `self.GameOver` _returnvalue_3)
  (bind _returnvalue_4 (`|CreateWidget` "/Game/Assets/UMG/FPSHUD_bp.FPSHUD_bp_C"))
  (bind _output_get (set `self.HUD` _returnvalue_4))
  (`UserWidget.AddToViewport` _output_get 0))

(event `self.ReceiveActorBeginOverlap`
  (params (OtherActor :type "Actor Object Reference"))
  (bind _asbase_door (cast `/Game/Assets/Blueprints/Rooms/Doors/BaseDoor` OtherActor)
    (:`then`
      (set `self.Door` _asbase_door))
    (:`CastFailed`
      (bind _asweapon_shop_bp (cast `/Game/Assets/Blueprints/Weapons/WeaponShop_bp` OtherActor)
        (:`then`
          (set `self.Shop` _asweapon_shop_bp))
        (:`CastFailed`
          (bind _asescape (cast `/Game/Assets/Blueprints/Escape` OtherActor))
          (set `self.Escape` _asescape))))))

(event `self.ReceiveActorEndOverlap`
  (params (OtherActor :type "Actor Object Reference"))
  (cast `/Game/Assets/Blueprints/Rooms/Doors/BaseDoor` OtherActor
    (:`then`
      (set `self.Door` (`self.NULLDOOR`)))
    (:`CastFailed`
      (cast `/Game/Assets/Blueprints/Weapons/WeaponShop_bp` OtherActor
        (:`then`
          (set `self.Shop` (`self.NULLSHOP`)))
        (:`CastFailed`
          (cast `/Game/Assets/Blueprints/Escape` OtherActor)
          (set `self.Escape` (`self.ESCAPENULL`)))))))

(event `self.ReceiveTick`
  (params (DeltaSeconds :type "Float (single-precision)"))
  (bind _healcurrent (`self.HealCurrent`))
  (bind _powerups (`self.Powerups`))
  (bind _powerups_2 (`self.Powerups`))
  (bind _powerups_3 (`self.Powerups`))
  (bind _returnvalue (`KismetMathLibrary.FTrunc` (`KismetMathLibrary.MultiplyMultiply_FloatFloat` 2.0)))
  (bind _returnvalue_2 (`KismetMathLibrary.FTrunc` (`KismetMathLibrary.MultiplyMultiply_FloatFloat` 2.0 1.0)))
  (bind _returnvalue_3 (`KismetMathLibrary.FTrunc` (`KismetMathLibrary.MultiplyMultiply_FloatFloat` 2.0 2.0)))
  (`|ExecutionSequence`
    (:`then_0`
      (if (`self.Firing`)
        (`Weapon.Fire` (`self.HeldWeapon`) (`self.TriggerPulled`))
        (`/Game/Assets/UMG/FPSHUD_bp.IsLow` (`self.HUD`))))
    (:`then_1`
      (set `self.TriggerPulled` false))
    (:`then_2`
      (if (<= _healcurrent 0.0)
        (`self.TakeDamage` -10.0)
        (else
          (set `self.HealCurrent` (- _healcurrent DeltaSeconds)))))
    (:`then_3`
      (`|ExecutionSequence`
        (:`then_0`
          (if (> (`KismetMathLibrary.And_IntInt` _powerups_2 _returnvalue) 0)
            (`KismetSystemLibrary.Delay` 30.0)
            (set `self.Powerups` (`KismetMathLibrary.Xor_IntInt` _powerups_2 _returnvalue))))
        (:`then_1`
          (if (> (`KismetMathLibrary.And_IntInt` _powerups_3 _returnvalue_2) 0)
            (`KismetSystemLibrary.Delay` 15.0)
            (set `self.Powerups` (`KismetMathLibrary.Xor_IntInt` _powerups_3 _returnvalue_2))))
        (:`then_2`
          (if (> (`KismetMathLibrary.And_IntInt` _powerups _returnvalue_3) 0)
            (`KismetSystemLibrary.Delay` 10.0)
            (set `self.Powerups` (`KismetMathLibrary.Xor_IntInt` _powerups _returnvalue_3))))))))

(event `InputAction|Pause`
  (params (Key :type "Key Structure"))
  (:`Pressed`
    (`UserWidget.AddToViewport` (`self.PauseMenu`) 0)))

(event `InputAction|Fire`
  (params (Key :type "Key Structure"))
  (:`Pressed`
    (set `self.Firing` true)
    (set `self.TriggerPulled` true))
  (:`Released`
    (set `self.Firing` false)))

(event `InputAction|KeyboardWeapon1`
  (params (Key :type "Key Structure"))
  (:`Pressed`
    (`self.SwitchWeapon1`)))

(event `Key|H`
  (params (Key :type "Key Structure"))
  (:`Pressed`
    (`self.KeyActive`)))

(event `InputAction|KeyboardWeapon2`
  (params (Key :type "Key Structure"))
  (:`Pressed`
    (`self.SwitchWeapon2`)))

(event `InputAction|KeyboardSideArm`
  (params (Key :type "Key Structure"))
  (:`Pressed`
    (`self.SwitchSideArm`)))

(event `InputAction|ControllerNextWeapon`
  (params (Key :type "Key Structure"))
  (bind _weaponindex (`self.WeaponIndex`))
  (:`Pressed`
    (`self.WrapAroundP` _weaponindex)
    (switch `int` _weaponindex :!label _label
      (:`0`
        (`self.SwitchSideArm`))
      (:`1`
        (`self.SwitchWeapon1`))
      (:`2`
        (`self.SwitchWeapon2`)))))

(event `InputAction|ControllerPrevWeapon`
  (params (Key :type "Key Structure"))
  (:`Pressed`
    (`self.WrapAroundN` (`self.WeaponIndex`))
    (goto _label)))

(event `InputAction|Interact`
  (params (Key :type "Key Structure"))
  (bind _deadends (`self.DeadEnds`))
  (bind _hallways (`self.Hallways`))
  (bind _weapons (`self.Weapons`))
  (bind _weaponclass (`WeaponShop.WeaponClass` (`self.CurrentWeaponShop`)))
  (bind _price (`WeaponShop.Price` (`self.CurrentWeaponShop`)))
  (bind _price_2 (`WeaponShop.Price` (`self.CurrentWeaponShop`)))
  (bind _returnvalue (/ (`WeaponShop.Price` (`self.CurrentWeaponShop`)) 2))
  (:`Pressed`
    (if (`self.AtDoor`)
      (bind _asbase_door (cast `/Game/Assets/Blueprints/Rooms/Doors/BaseDoor` (`|GetArrayItem` (`self.GetOverlappingActors` "/Game/Assets/Blueprints/Rooms/Doors/BaseDoor.BaseDoor_C"))))
      (if (not (`/Game/Assets/Blueprints/Rooms/Doors/BaseDoor.Locked` _asbase_door))
        (`self.Transaction` (`/Game/Assets/Blueprints/Rooms/Doors/BaseDoor.Cost` _asbase_door))
        (bind _result (`/Engine/EditorBlueprintResources/StandardMacros.IncrementInt` (`self.Spawns`))
          (:`  `
            (set `/Game/Assets/Blueprints/Rooms/Doors/BaseDoor.Opening` true _asbase_door)
            (set `self.AtDoor` false)
            (if (== (mod _result 3) 0)
              (bind _returnvalue_2 (`SceneComponent.K2_GetComponentToWorld` (`/Game/Assets/Blueprints/Rooms/Doors/BaseDoor.Forward` _asbase_door)))
              (`|SpawnActorFromClass` (`|GetArrayItem` _deadends (`KismetMathLibrary.RandomInteger` (`KismetArrayLibrary.Array_Length` _deadends))) _returnvalue_2 "Undefined" "OverrideRootScale" null null)
              (else
                (`|SpawnActorFromClass` (`|GetArrayItem` _hallways (`KismetMathLibrary.RandomInteger` (`KismetArrayLibrary.Array_Length` _hallways))) _returnvalue_2 "Undefined" "OverrideRootScale" null null))))))
      (elif (`self.AtShop`)
        (bind _asweapon_shop_bp (cast `/Game/Assets/Blueprints/Weapons/WeaponShop_bp` (`|GetArrayItem` (`self.GetOverlappingActors` "/Game/Assets/Blueprints/Weapons/WeaponShop_bp.WeaponShop_bp_C"))))
        (bind _output_get (set `self.CurrentWeaponShop` _asweapon_shop_bp))
        (if (`.IsSideArm` (defaults `/Game/Assets/Blueprints/FPSCharacter_bp` (`WeaponShop.WeaponClass` _output_get)))
          (if (== (`GameplayStatics.GetObjectClass` (`self.SideArm`)) (`WeaponShop.WeaponClass` (`self.CurrentWeaponShop`)))
            _
            (elif (<= _price_2 (`self.Cash`))
              (`self.Transaction` _price_2)
              (bind _returnvalue_3 (`|SpawnActorFromClass` (`WeaponShop.WeaponClass` (`self.CurrentWeaponShop`)) (`self.GetTransform`) "AlwaysSpawn" "OverrideRootScale" null null))
              (`self.EquipSideArm` _returnvalue_3)))
          (elif (or (== (`GameplayStatics.GetObjectClass` (`|GetArrayItem` _weapons)) _weaponclass) (== _weaponclass (`GameplayStatics.GetObjectClass` (`|GetArrayItem` _weapons 1))))
            (if (<= _returnvalue (`self.Cash`))
              (`self.Transaction` _returnvalue)
              (for _array_element (`self.Weapons`)
                (if (== (`GameplayStatics.GetObjectClass` _array_element) (`WeaponShop.WeaponClass` (`self.CurrentWeaponShop`)))
                  (set `Weapon.AmmoCurrent` (`Weapon.AmmoMax` _array_element) _array_element)
                  (break))))
            (else
              (for (_array_element_2 _array_index) (`self.Weapons`)
                (if (== _array_element_2 null)
                  (set `self.ReplaceIndex` _array_index)
                  (break)
                  (else
                    (set `self.ReplaceIndex` (`self.CurrentWeapon`)))))
              (if (<= _price (`self.Cash`))
                (`self.Transaction` _price)
                (bind _returnvalue_4 (`|SpawnActorFromClass` (`WeaponShop.WeaponClass` (`self.CurrentWeaponShop`)) (`self.GetTransform`) "AlwaysSpawn" "OverrideRootScale" null null))
                (`self.EquipWeapon` _returnvalue_4 (`self.ReplaceIndex`))))))
        (elif (`self.AtKey`)
          (bind _askeystone (cast `/Game/Assets/Blueprints/Keystone` (`|GetArrayItem` (`self.GetOverlappingActors` "/Game/Assets/Blueprints/Keystone.Keystone_C"))))
          (`SceneComponent.ToggleVisibility` (`/Game/Assets/Blueprints/Keystone.Light` _askeystone) false)
          (set `self.AtKey` false)
          (`self.KeyActive`)
          (elif (`self.AtExit`)
            (bind _asescape (cast `/Game/Assets/Blueprints/Escape` (`|GetArrayItem` (`self.GetOverlappingActors` "/Game/Assets/Blueprints/Escape.Escape_C"))))
            (if (== (`/Game/Assets/Blueprints/Escape.Count` _asescape) 3)
              (`UserWidget.AddToViewport` (`self.Complete`) 0))))))))

(fn `TakeDamage`
  (params (Damage :type "Float (double-precision)"))
  (set `self.HealCurrent` (`self.HealInterval`))
  (bind _output_get (set `self.Health` (`KismetMathLibrary.FClamp` (- (`self.Health`) Damage) 0.0 (`self.MaxHealth`))))
  (if (<= _output_get 0.0)
    (`UserWidget.AddToViewport` (`self.GameOver`) 0)
    (else
      (`self.UpdateHealth` _output_get))))

(fn `Transaction`
  (params (Cost :type Integer))
  (if (< Cost 0)
    (if (> (`KismetMathLibrary.And_IntInt` (`KismetMathLibrary.FTrunc` (`KismetMathLibrary.MultiplyMultiply_FloatFloat` 2.0)) (`self.Powerups`)) 0)
      (bind _output_get (set `self.Cash` (- (`self.Cash`) (* Cost 2))))
      (`self.UpdateCash` _output_get)
      (else
        (bind _output_get_2 (set `self.Cash` (- (`self.Cash`) Cost) :!label _label))
        (`self.UpdateCash` _output_get_2)))
    (elif (> (`KismetMathLibrary.And_IntInt` (`KismetMathLibrary.FTrunc` (`KismetMathLibrary.MultiplyMultiply_FloatFloat` 2.0 1.0)) (`self.Powerups`)) 0)
      (bind _output_get_3 (set `self.Cash` (- (`self.Cash`) (/ Cost 2))))
      (`self.UpdateCash` _output_get_3)
      (else
        (goto _label)))))

(fn `UserConstructionScript`
  (set `self.DeadEnds` (`|MakeArray` "/Game/Assets/Blueprints/Rooms/DeadEnds/Room1.Room1_C" "/Game/Assets/Blueprints/Rooms/DeadEnds/Room2.Room2_C" :!type "/Game/Assets/Blueprints/Rooms/DeadEnds/BaseRoom Class Reference"))
  (set `self.Hallways` (`|MakeArray` "/Game/Assets/Blueprints/Rooms/Hallways/Hallway1.Hallway1_C" "/Game/Assets/Blueprints/Rooms/Hallways/Hallway2.Hallway2_C" "/Game/Assets/Blueprints/Rooms/Hallways/Hallway3.Hallway3_C" "/Game/Assets/Blueprints/Rooms/Hallways/Hallway4.Hallway4_C" "/Game/Assets/Blueprints/Rooms/Hallways/Hallway5.Hallway5_C" :!type "/Game/Assets/Blueprints/Rooms/Hallways/BaseHallway Class Reference"))
  (set `self.Meshes` (`|MakeArray` "/Game/Assets/Mesh/moneys.moneys" "/Game/Assets/Mesh/moneym.moneym" "/Game/Assets/Mesh/moneyl.moneyl" :!type "StaticMesh Object Reference"))
  (set `self.Values` (`|MakeArray` -100 -300 -500)))

(fn `WrapAroundN`
  (params (A :type Integer))
  (bind _returnvalue (- A 1))
  (if (< _returnvalue 0)
    (set `self.WeaponIndex` 2)
    (else
      (set `self.WeaponIndex` _returnvalue))))

(fn `WrapAroundP`
  (params (A :type Integer))
  (set `self.WeaponIndex` (mod (+ A 1) 3)))